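; Weather controller Blueprint that spins the sun light every tick and switches randomly between sunny, rain and dust on right mouse click.
; Each switch rerolls until the weather differs, stops the old rain or dust particles, then timeline-blends sky, cloud and light parameters between presets.
; Delays stagger particle changes against the blend.
; Rain also ramps WaterAmount on a dynamic ground material created in the construction script.
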(event Custom|Weather
  (bind _dustref (Variables|Default|GetDustRef))
  (bind _rainref (Variables|Default|GetRainRef))
  (bind _skyref (Variables|Default|GetSkyRef))
  (bind _particlesystemcomponent (Variables|/Script/Engine.Emitter|GetParticleSystemComponent _rainref))
  (bind _particlesystemcomponent_2 (Variables|/Script/Engine.Emitter|GetParticleSystemComponent _dustref))
  (if (Utilities|IsValid (Variables|Default|GetSkyRef))
    (bind _output_get (Variables|Default|SetPostWeather (Math|Random|RandomIntegerinRange 0 2) :!label _label))
    (if (== (Variables|Default|GetPreWeather) _output_get)
      (goto _label)
      (else
        (switch int _output_get
          (:Default
            (Variables|Default|SetPostParam (Variables|Default|GetSunny))
            (Variables|Default|SetWaterAmount 0.0))
          (:0
            (Variables|Default|SetPostParam (Variables|Default|GetRain))
            (Variables|Default|SetWaterAmount 4.0))
          (:1
            (Variables|Default|SetPostParam (Variables|Default|GetDust))
            (Variables|Default|SetWaterAmount 0.0)))
        (switch int (Variables|Default|GetPreWeather)
          (:Default
            (Utilities|FlowControl|Sequence :!label _label_2
              (:then_0
                (bind _newtrack_0 (Timeline|Timeline_0 PlayFromStart)
                  (:Update
                    (Variables|/Engine/EngineSky/BP_Sky_Sphere.BP_Sky_Sphere_C|Setalpha _skyref (.alpha (Utilities|Struct|BreakWheaterParamBP (Variables|Default|GetPostParam))))
                    (Variables|/Engine/EngineSky/BP_Sky_Sphere.BP_Sky_Sphere_C|SetZenith%20color%20W _skyref (Math|Color|Lerp(LinearColor) (.ZenithColor (Utilities|Struct|BreakWheaterParamBP (Variables|Default|GetPreParam))) (.ZenithColor (Utilities|Struct|BreakWheaterParamBP (Variables|Default|GetPostParam))) _newtrack_0))
                    (Variables|/Engine/EngineSky/BP_Sky_Sphere.BP_Sky_Sphere_C|SetHorizon%20color%20W _skyref (Math|Color|Lerp(LinearColor) (.HorizonColor (Utilities|Struct|BreakWheaterParamBP (Variables|Default|GetPreParam))) (.HorizonColor (Utilities|Struct|BreakWheaterParamBP (Variables|Default|GetPostParam))) _newtrack_0))
                    (Variables|/Engine/EngineSky/BP_Sky_Sphere.BP_Sky_Sphere_C|SetCloud%20color%20W _skyref (Math|Color|Lerp(LinearColor) (.CloudColor (Utilities|Struct|BreakWheaterParamBP (Variables|Default|GetPreParam))) (.CloudColor (Utilities|Struct|BreakWheaterParamBP (Variables|Default|GetPostParam))) _newtrack_0))
                    (Rendering|Material|SetScalarParameterValue (Variables|/Engine/EngineSky/BP_Sky_Sphere.BP_Sky_Sphere_C|GetSky%20material _skyref) "Cloud Opacity" (Math|Float|Lerp (.CloudOpacity (Utilities|Struct|BreakWheaterParamBP (Variables|Default|GetPreParam))) (.CloudOpacity (Utilities|Struct|BreakWheaterParamBP (Variables|Default|GetPostParam))) _newtrack_0) :!class /Script/Engine.MaterialInstanceDynamic)
                    (Rendering|Components|Light|SetLightColor (Variables|/Script/Engine.Light|GetLightComponent (Variables|Default|GetLightRef)) (Math|Color|Lerp(LinearColor) (.LightColor (Utilities|Struct|BreakWheaterParamBP (Variables|Default|GetPreParam))) (.LightColor (Utilities|Struct|BreakWheaterParamBP (Variables|Default|GetPostParam))) _newtrack_0) true))
                  (:Finished
                    (Variables|Default|SetPreWeather (Variables|Default|GetPostWeather))
                    (Variables|Default|SetPreParam (Variables|Default|GetPostParam)))))
              (:then_1
                (Utilities|FlowControl|Delay 3.0)
                (switch int (Variables|Default|GetPostWeather)
                  (:0
                    (Components|Activation|Activate _particlesystemcomponent false)
                    (bind _newtrack_0_2 (Timeline|Timeline_1 PlayFromStart)
                      (:Update
                        (Rendering|Material|SetScalarParameterValue (Variables|Default|GetGroundMat) "WaterAmount" (Math|Float|Lerp 1.2 4.0 _newtrack_0_2) :!class /Script/Engine.MaterialInstanceDynamic))))
                  (:1
                    (Components|Activation|Activate _particlesystemcomponent_2 false))))))
          (:0
            (Components|Activation|Deactivate _particlesystemcomponent)
            (Utilities|FlowControl|Sequence
              (:then_0
                (bind _newtrack_0_3 (Timeline|Timeline_2 PlayFromStart)
                  (:Update
                    (Rendering|Material|SetScalarParameterValue (Variables|Default|GetGroundMat) "WaterAmount" (Math|Float|Lerp 4.0 1.2 _newtrack_0_3) :!class /Script/Engine.MaterialInstanceDynamic))))
              (:then_1
                (Utilities|FlowControl|Delay 3.0 :!label _label_3)
                (goto _label_2))))
          (:1
            (Components|Activation|Deactivate _particlesystemcomponent_2)
            (goto _label_3)))))))

(event EventTick
  (params (DeltaSeconds :type Float%20%28single-precision%29))
  (Transformation|AddActorLocalRotation (Variables|Default|GetLightRef) (Math|Rotator|MakeRotator 0.0 (* DeltaSeconds 3e+01) 0.0) false false)
  (Default|UpdateSunDirection (Variables|Default|GetSkyRef)))

(event EventBeginPlay
  (Variables|Default|SetPreParam (Variables|Default|GetSunny)))

(event Input|MouseEvents|RightMouseButton
  (params (Key :type Key%20Structure :default "None"))
  (:Pressed
    (CallFunction|Weather)))

(fn ConstructionScript
  (bind _returnvalue (Rendering|Material|CreateDynamicMaterialInstance (Variables|Default|GetGroundRef) "None" "None" :!class /Script/Engine.KismetMaterialLibrary))
  (Variables|Default|SetGroundMat _returnvalue))