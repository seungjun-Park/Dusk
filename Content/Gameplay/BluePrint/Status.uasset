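; Status holds one typed gameplay stat with minimum, current and maximum values, exposed through getters.
; Init sets the type, bounds, starting value and increase rate only once, guarded by an initialized flag.
; Update grows the maximum by the increase rate, compounding on each call, and leaves the current value untouched.
; SetCurrentStatus ignores values outside the bounds instead of clamping them.
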(fn Init
  (params (statusType :type StatusType%20Enum :default "NewEnumerator20") (minStatus :type Float%20%28single-precision%29) (currentStatus :type Float%20%28single-precision%29) (maxStatus :type Float%20%28single-precision%29) (increaseRate :type Float%20%28single-precision%29))
  (if (not (Variables|Private|GetisInitialized))
    (Variables|private|SetstatusType statusType)
    (Variables|private|SetminStatus minStatus)
    (Variables|Private|SetcurrentStatus currentStatus)
    (Variables|Private|SetmaxStatus maxStatus)
    (Variables|Private|SetincreaseRate increaseRate)
    (Variables|Private|SetisInitialized true)))

(fn Update
  (Variables|Private|SetmaxStatus (+ (Variables|Private|GetmaxStatus) (* (Variables|Private|GetmaxStatus) (Variables|Private|GetincreaseRate)))))

(fn SetCurrentStatus
  (params (value :type Float%20%28single-precision%29))
  (if (and (>= value (Variables|private|GetminStatus)) (<= value (Variables|Private|GetmaxStatus)))
    (Variables|Private|SetcurrentStatus value)))

(fn GetCurrentStatus
  (return (Variables|Private|GetcurrentStatus)))

(fn GetMaxStatus
  (return (Variables|Private|GetmaxStatus)))

(fn GetMinStatus
  (return (Variables|private|GetminStatus)))

(fn GetStatusType
  (return (Variables|private|GetstatusType)))